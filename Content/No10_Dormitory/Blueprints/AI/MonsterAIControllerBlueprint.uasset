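; AI controller for the dormitory monster, which patrols, chases the player and triggers death at close range via a console event.
; RunAI loops moves to randomized offsets from random PTP-tagged points and starts a timer that repeats SendLine's trace sweep.
; A player hit starts a chase or a move to the player's position, depending on the monster's particle state.
; ComplexAIMovement, uncalled here, changes floors by respawning the monster.
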(event `RunAI`
  (params (CurrectDestFloor :type Integer))
  (if (not (`self.IfCatching`))
    (set `self.CurrentDestFloor` CurrectDestFloor)
    (if (not (`KismetSystemLibrary.K2_TimerExists` null "SendLineForSearch"))
      (`KismetSystemLibrary.K2_SetTimer` null "SendLineForSearch" 0.1 true))
    (bind _location (`self.MonsterMove`))
    (`|AIMoveTo` (`self.K2_GetPawn`) _location
      (:`OnSuccess`
        _)
      (:`OnFail`
        _))
    (if (not (`self.IfCatching`))
      (`self.RunAI` 0))))

(event `self.ReceiveTick`
  (params (DeltaSeconds :type "Float (single-precision)"))
  (bind (_outactors _returnvalue) (`KismetSystemLibrary.SphereOverlapActors_NEW` (`self.K2_GetActorLocation` (`self.K2_GetPawn`)) 100.0 (`|MakeArray` "ObjectTypeQuery3" :!type "EObjectTypeQuery Enum") "/Game/No10_Dormitory/Blueprints/ObjectBlueprints/MyCharacterBlueprint.MyCharacterBlueprint_C"))
  (if _returnvalue
    (`KismetSystemLibrary.ExecuteConsoleCommand` "ce DIE")))

(event `b`
  (if (not (`self.IfCatching`))
    (set `self.IfCatching` true)
    (`|AIMoveTo` (`self.K2_GetPawn`) (0.0 0.0 0.0) (`GameplayStatics.GetPlayerPawn` 0)
      (:`OnSuccess`
        _)
      (:`OnFail`
        _))
    (if (`self.IfCatching`)
      (bind (_outactors _returnvalue) (`KismetSystemLibrary.SphereOverlapActors_NEW` (`self.K2_GetActorLocation`) 100.0 (`|MakeArray` "ObjectTypeQuery3" :!type "EObjectTypeQuery Enum") "/Game/No10_Dormitory/Blueprints/ObjectBlueprints/MyCharacterBlueprint.MyCharacterBlueprint_C"))
      (if _returnvalue
        (`KismetSystemLibrary.ExecuteConsoleCommand` "ce DIE")
        (else
          (set `self.IfCatching` false)
          (`self.RunAI` 0))))))

(event `MovetoLastL`
  (set `self.IfCatching` false)
  (`|AIMoveTo` (`self.K2_GetPawn`) (`self.K2_GetActorLocation` (`GameplayStatics.GetPlayerPawn` 0))
    (:`OnSuccess`
      _)
    (:`OnFail`
      _))
  (`self.RunAI` 0))

(fn `MonsterMove`
  (returns (Location :type "Vector Structure"))
  (bind _outactors (`GameplayStatics.GetAllActorsWithTag` (`KismetStringLibrary.Conv_StringToName` (`KismetStringLibrary.Concat_StrStr` "PTP" (`KismetStringLibrary.Conv_IntToString` (`KismetMathLibrary.RandomIntegerInRange` 1 7))))))
  (return (`KismetMathLibrary.MakeVector` (+ (.x (`self.K2_GetActorLocation` (`KismetArrayLibrary.Array_Get` _outactors))) (`KismetMathLibrary.RandomFloatInRange` -100.0 100.0)) (+ (.y (`self.K2_GetActorLocation` (`KismetArrayLibrary.Array_Get` _outactors))) (`KismetMathLibrary.RandomFloatInRange` -10000.0 500.0)) (.z (`self.K2_GetActorLocation` (`KismetArrayLibrary.Array_Get` _outactors))))))

(fn `SendLineForSearch`
  (`self.SendLine`))

(fn `UserConstructionScript`)