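; First-person player character with mouse look, walking, sprinting, an animated dimmable flashlight and climbing.
; A looping camera trace notifies faced actors through PickupInterface; holding Space against any hit disables gravity and moves up, with a RadialForce impulse on exit.
; Sprinting widens FOV, while movement input drives footstep audio, sprint camera shake and timers that gradually lower max speed while running, restoring it otherwise.
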(event `OpenFlashLightAnime`
  (`SceneComponent.SetVisibility` (`self.SpotLight`) true false)
  (set `self.IsFlashAnime` true)
  (bind (_direction _updowny _leftrightz) (`Timeline|TimelineOpenFlashLightAnime` :!via `PlayFromStart`)
    (:`Update`
      (`SceneComponent.K2_SetRelativeRotation` (`self.sdt`) (`KismetMathLibrary.MakeRotator` 0.0 _updowny _leftrightz) false false))
    (:`Finished`
      (set `self.IsFlashAnime` false))))

(event `CloseFlashLightAnime`
  (set `self.IsFlashAnime` true)
  (bind (_direction _updowny _leftrightz) (`Timeline|TimelineCloseFlashLightAnime` :!via `PlayFromStart`)
    (:`Update`
      (`SceneComponent.K2_SetRelativeRotation` (`self.sdt`) (`KismetMathLibrary.MakeRotator` 0.0 _updowny _leftrightz) false false))
    (:`Finished`
      (set `self.IsFlashAnime` false)
      (`SceneComponent.SetVisibility` (`self.SpotLight`) false false))))

(event `Key|SpaceBar`
  (params (Key :type "Key Structure" :default "AnyKey"))
  (:`Pressed`
    (set `self.Climbing` true))
  (:`Released`
    (set `self.Climbing` false)))

(event `Key|F`
  (params (Key :type "Key Structure" :default "AnyKey"))
  (:`Pressed`
    (if (not (`self.IsFlashAnime`))
      (`/Engine/EditorBlueprintResources/StandardMacros.FlipFlop`
        (:`A`
          (`self.CloseFlashLightAnime`))
        (:`B`
          (`self.OpenFlashLightAnime`))))))

(event `Key|LeftShift`
  (params (Key :type "Key Structure" :default "AnyKey"))
  (bind _camera (`self.Camera`))
  (bind _fieldofview (`CameraComponent.FieldOfView` _camera))
  ;[1 1 1] 跑步走+视野变换
  (:`Pressed`
    (set `self.IsRunning` true)
    (set `self.RunningScale` 3.0)
    (`|ExecutionSequence`
      (:`then_0`
        (goto _label_2 :!via `Break`))
      (:`then_1`
        (bind _index (`/Game/No10_Dormitory/Blueprints/MacroLibrary.ForLoopWithDelay` (`KismetMathLibrary.FTrunc` _fieldofview) 105 0.01 :!label _label)
          (:`LoopBody`
            (`CameraComponent.SetFieldOfView` _camera (`KismetMathLibrary.Conv_IntToDouble` _index)))))))
  (:`Released`
    (set `self.IsRunning` false)
    (`|ExecutionSequence`
      (:`then_1`
        (set `self.RunningScale` 1.0)
        (`|ExecutionSequence`
          (:`then_0`
            (goto _label :!via `Break`))
          (:`then_1`
            (bind _index_2 (`/Game/No10_Dormitory/Blueprints/MacroLibrary.ForLoopWithDelay` (- 105 (`KismetMathLibrary.FTrunc` _fieldofview)) 15 0.01 :!label _label_2)
              (:`LoopBody`
                (`CameraComponent.SetFieldOfView` _camera (`KismetMathLibrary.Conv_IntToDouble` (+ (- 15 _index_2) 90)))))))))))

(event `InputAxis|FlashLighting`
  (params (AxisValue :type "Float (single-precision)"))
  (bind _returnvalue (+ AxisValue (`LightComponentBase.Intensity` (`self.SpotLight`))))
  ;[1 1 1] 手电筒亮度
  (if (and (> _returnvalue 0.0) (< _returnvalue 5000.0))
    (`LightComponent.SetIntensity` (`self.SpotLight`) _returnvalue)))

(event `SexGirl`
  (set `self.IsGirlSexy` true))

(event `self.ReceiveBeginPlay`
  (`KismetSystemLibrary.K2_SetTimer` null "SendLine" 0.1 true))

(event `Key|LeftMouseButton`
  (params (Key :type "Key Structure" :default "AnyKey"))
  (:`Pressed`
    (set `self.DrawDebugLine` true))
  (:`Released`
    (set `self.DrawDebugLine` false)))

(event `InputAxis|Forword`
  (params (AxisValue :type "Float (single-precision)"))
  (bind (_returnvalue_roll _returnvalue_pitch _returnvalue_yaw) (`KismetMathLibrary.BreakRotator` (`self.GetControlRotation`)))
  (bind _returnvalue (`KismetMathLibrary.GetForwardVector` (`KismetMathLibrary.MakeRotator` 0.0 0.0 _returnvalue_yaw)))
  ;[1 1 1] 移动
  (if (`self.IsRunning`)
    (`self.AddMovementInput` _returnvalue (* 3 AxisValue))
    (else
      (`self.AddMovementInput` _returnvalue AxisValue)))
  ;[1 1 1] 脚步声
  (`self.WalkSound` AxisValue (stale `InputAxis|Right` AxisValue) :!label _label_3
    (:`Out`
      (`self.TimerForRun` AxisValue (stale `InputAxis|Right` AxisValue)))))

(event `InputAxis|ViewX`
  (params (AxisValue :type "Float (single-precision)"))
  ;[1 1 1] 视角
  (`self.AddControllerYawInput` AxisValue))

(event `InputAxis|ViewY`
  (params (AxisValue :type "Float (single-precision)"))
  (bind _returnvalue (+ (.pitch (.rotation (`SceneComponent.GetRelativeTransform` (`self.Camera`)))) AxisValue))
  ;[1 1 1] 视角
  (if (not (or (> _returnvalue 60.0) (< _returnvalue -60.0)))
    (`SceneComponent.K2_AddRelativeRotation` (`self.Camera`) (`KismetMathLibrary.MakeRotator` 0.0 AxisValue) false false)
    (`SceneComponent.K2_AddRelativeRotation` (`self.sdt`) (`KismetMathLibrary.MakeRotator` 0.0 (* AxisValue -0.5)) false false)))

(event `InputAxis|Right`
  (params (AxisValue :type "Float (single-precision)"))
  (bind (_returnvalue_roll _returnvalue_pitch _returnvalue_yaw) (`KismetMathLibrary.BreakRotator` (`self.GetControlRotation`)))
  (bind _returnvalue (`KismetMathLibrary.GetRightVector` (`KismetMathLibrary.MakeRotator` 0.0 0.0 _returnvalue_yaw)))
  ;[1 1 1] 移动
  (if (`self.IsRunning`)
    (`self.AddMovementInput` _returnvalue (* (`self.RunningScale`) AxisValue))
    (goto _label_3)
    (else
      (`self.AddMovementInput` _returnvalue AxisValue)
      (goto _label_3))))

(fn `Climb`
  (`self.K2_AddActorLocalTransform` (`KismetMathLibrary.MakeTransform` (0.0 0.0 10.0))))

(fn `SendLine`
  (bind _camera (`self.Camera`))
  (bind _lastfacedactor (`self.LastFacedActor`))
  (bind _lastfacedactor_2 (`self.LastFacedActor`))
  (bind _charactermovement (`self.CharacterMovement`))
  (bind _returnvalue (`SceneComponent.K2_GetComponentLocation` _camera))
  (bind _returnvalue_2 (+ _returnvalue (* (`SceneComponent.GetForwardVector` _camera) 100)))
  (if (`self.DrawDebugLine`)
    (bind (_outhit _returnvalue_3) (`KismetSystemLibrary.LineTraceSingle` :`Start` _returnvalue :`End` _returnvalue_2 :`TraceChannel` "TraceTypeQuery1" :`DrawDebugType` "Persistent" :`DrawTime` 1.0))
    (if _returnvalue_3
      (if (not (== (`.HitActor` (`GameplayStatics.BreakHitResult` _outhit)) _lastfacedactor_2))
        (message `/Game/No10_Dormitory/Blueprints/PickupsInterface.PickupInterface_ChangeFaceAtObject` _lastfacedactor_2 false)
        (message `/Game/No10_Dormitory/Blueprints/PickupsInterface.PickupInterface_ChangeFaceAtObject` (`.HitActor` (`GameplayStatics.BreakHitResult` _outhit)) true)
        (set `self.LastFacedActor` (`.HitActor` (`GameplayStatics.BreakHitResult` _outhit))))
      (if (`self.Climbing`) :!label _label
        (set `CharacterMovementComponent.GravityScale` 0.0 _charactermovement)
        (bind _output_get (set `self.IsNearClimb` true))
        (if (not (`KismetSystemLibrary.K2_IsTimerActive` null "Climb"))
          (`KismetSystemLibrary.K2_SetTimer` null "Climb" 0.02 true))
        (else
          (set `CharacterMovementComponent.GravityScale` 1.0 _charactermovement :!label _label_2)
          (`KismetSystemLibrary.K2_ClearTimer` null "Climb")
          (if _output_get
            (`RadialForceComponent.FireImpulse` (`self.RadialForce`)))
          (set `self.IsNearClimb` false)))
      (else
        (message `/Game/No10_Dormitory/Blueprints/PickupsInterface.PickupInterface_ChangeFaceAtObject` _lastfacedactor_2 false)
        (set `self.LastFacedActor` null)
        (goto _label_2)))
    (else
      (bind (_outhit_2 _returnvalue_4) (`KismetSystemLibrary.LineTraceSingle` :`Start` _returnvalue :`End` _returnvalue_2 :`TraceChannel` "TraceTypeQuery1" :`DrawTime` 1.0))
      (if _returnvalue_4
        (if (== (`.HitActor` (`GameplayStatics.BreakHitResult` _outhit_2)) _lastfacedactor)
          (goto _label)
          (else
            (message `/Game/No10_Dormitory/Blueprints/PickupsInterface.PickupInterface_ChangeFaceAtObject` _lastfacedactor false)
            (message `/Game/No10_Dormitory/Blueprints/PickupsInterface.PickupInterface_ChangeFaceAtObject` (`.HitActor` (`GameplayStatics.BreakHitResult` _outhit_2)) true)
            (set `self.LastFacedActor` (`.HitActor` (`GameplayStatics.BreakHitResult` _outhit_2)))
            (goto _label)))
        (else
          (message `/Game/No10_Dormitory/Blueprints/PickupsInterface.PickupInterface_ChangeFaceAtObject` _lastfacedactor false)
          (set `self.LastFacedActor` null)
          (goto _label_2))))))

(fn `TimerToAddMaxSpeed`
  (bind _charactermovement (`self.CharacterMovement`))
  (bind _returnvalue (+ (`CharacterMovementComponent.MaxWalkSpeed` _charactermovement) 1.0))
  (if (< _returnvalue 600.0)
    (set `CharacterMovementComponent.MaxWalkSpeed` _returnvalue _charactermovement)
    (else
      (`KismetSystemLibrary.K2_ClearTimer` null "TimerToAddMaxSpeed"))))

(fn `TimerToSubMaxSpeed`
  (bind _charactermovement (`self.CharacterMovement`))
  (bind _returnvalue (- (`CharacterMovementComponent.MaxWalkSpeed` _charactermovement) 1.0))
  (if (> _returnvalue 200.0)
    (set `CharacterMovementComponent.MaxWalkSpeed` _returnvalue _charactermovement)
    (else
      (`KismetSystemLibrary.K2_ClearTimer` null "TimerToSubMaxSpeed"))))

(fn `UserConstructionScript`)