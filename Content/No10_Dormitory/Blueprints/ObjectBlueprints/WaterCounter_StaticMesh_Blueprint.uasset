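; Dormitory water counter that the player toggles with the StudentCard pickup tag.
; The pickup interface enables input while the player faces it, so a left click can act on it.
; A click swaps StudentCard in the player's pickup tags for TagString and shows the StaticMesh, or swaps it back and hides the mesh.
; If neither tag is found or the counter is unusable, it shows the missing-card message.
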(event `/Game/No10_Dormitory/Blueprints/PickupsInterface.PickupInterface_ChangeFaceAtObject`
  (params (IsFaceing :type Boolean))
  (bind _returnvalue (`GameplayStatics.GetPlayerController` 0))
  (if IsFaceing
    (`self.EnableInput` _returnvalue)
    (`KismetSystemLibrary.PrintString` "In")
    (else
      (`self.DisableInput` _returnvalue)
      (`KismetSystemLibrary.PrintString` "Out"))))

(event `Key|LeftMouseButton`
  (params (Key :type "Key Structure" :default "AnyKey"))
  (:`Pressed`
    (if (`self.CanBeUsed`)
      (bind _findindex (`/Game/No10_Dormitory/Blueprints/GameMacro.FindIfPlayerHaveTag` "StudentCard")
        (:`Find`
          (bind _newparam (`/Game/No10_Dormitory/Blueprints/GameMacro.GetPickUpTags`)
            (:`Out`
              (`KismetArrayLibrary.Array_Set` _newparam _findindex (`self.TagString`))
              (`SceneComponent.SetVisibility` (`self.StaticMesh`) true false))))
        (:`Not`
          (bind _findindex_2 (`/Game/No10_Dormitory/Blueprints/GameMacro.FindIfPlayerHaveTag` (`self.TagString`))
            (:`Find`
              (bind _newparam_2 (`/Game/No10_Dormitory/Blueprints/GameMacro.GetPickUpTags`)
                (:`Out`
                  (`KismetArrayLibrary.Array_Set` _newparam_2 _findindex_2 "StudentCard")
                  (`SceneComponent.SetVisibility` (`self.StaticMesh`) false false))))
            (:`Not`
              (`/Game/No10_Dormitory/Blueprints/GameMacro.ShowMessage` (`self.MessageWhenDoesntHaveCard`) :!label _label)))))
      (else
        (goto _label)))))

(fn `UserConstructionScript`)