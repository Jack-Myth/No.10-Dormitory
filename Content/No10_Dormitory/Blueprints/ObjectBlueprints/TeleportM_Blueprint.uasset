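; Teleport marker actor that plays a sound and animates its mesh when Explan fires, and can be removed by the player.
; A timeline offsets the mesh's height from the Z cached in the construction script, while a Delay loop started from its update keeps the mesh spinning.
; The pickup interface's facing event toggles input, so a right-click while faced broadcasts a zero teleport point and destroys the actor.
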(event `/Game/No10_Dormitory/Blueprints/PickupsInterface.PickupInterface_ChangeFaceAtObject`
  (params (IsFaceing :type Boolean))
  (bind _returnvalue (`GameplayStatics.GetPlayerController` 0))
  (if IsFaceing
    (`self.EnableInput` _returnvalue)
    (else
      (`self.DisableInput` _returnvalue))))

(event `Explan`
  (bind (_returnvalue_x _returnvalue_y) (`KismetMathLibrary.BreakVector` (`SceneComponent.K2_GetComponentLocation` (`self.StaticMesh`))))
  (`GameplayStatics.PlaySoundAtLocation` "/Game/No10_Dormitory/Sound/科技.科技" (`self.K2_GetActorLocation`))
  (bind (_direction `_新建轨迹_0`) (`Timeline|时间轴_0`)
    (:`Update`
      (`SceneComponent.K2_SetWorldLocation` (`self.StaticMesh`) (`KismetMathLibrary.MakeVector` _returnvalue_x _returnvalue_y (+ (`self.LocationZ`) `_新建轨迹_0`)) true false)
      (`SceneComponent.K2_AddRelativeRotation` (`self.StaticMesh`) (struct :`Yaw` 3.6) false false :!label _label)
      (`KismetSystemLibrary.Delay` 0.01)
      (goto _label))))

(event `Key|RightMouseButton`
  (params (Key :type "Key Structure" :default "AnyKey"))
  (:`Pressed`
    (`self.SetTeleportMPoint` (0.0 0.0 0.0))
    (`self.K2_DestroyActor`)))

(fn `UserConstructionScript`
  (bind (_returnvalue_x _returnvalue_y _returnvalue_z) (`KismetMathLibrary.BreakVector` (`SceneComponent.K2_GetComponentLocation` (`self.StaticMesh`))))
  (set `self.LocationZ` _returnvalue_z))