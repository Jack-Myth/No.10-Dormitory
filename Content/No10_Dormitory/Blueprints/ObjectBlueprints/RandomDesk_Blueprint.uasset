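; Construction-script Blueprint that scatters desk static mesh components for the dormitory environment, with no active event graph logic.
; It loops over DeskCount, adding each mesh at a random position inside a RandomX by RandomY area centered on the actor, with random yaw.
; A RandomStream drives the placement, using derived seeds for X and Y.
; The ReRandom flag reseeds the stream on demand, then clears itself.
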(fn `UserConstructionScript`
  (bind _randomstream (`self.RandomStream`))
  (bind _returnvalue (/ (`self.RandomX`) 2.0))
  (bind _returnvalue_2 (/ (`self.RandomY`) 2.0))
  (bind _returnvalue_3 (`KismetMathLibrary.RandomIntegerInRangeFromStream` 0 1000 _randomstream))
  (if (`self.ReRandom`)
    (`KismetMathLibrary.SeedRandomStream` _randomstream)
    (set `self.ReRandom` false))
  (for _ (range (+ (`self.DeskCount`) 1))
    (set `self.TempTransform` (`KismetMathLibrary.MakeTransform` (`KismetMathLibrary.MakeVector` (`KismetMathLibrary.RandomFloatInRangeFromStream` (* -1 _returnvalue) _returnvalue (`KismetMathLibrary.MakeRandomStream` _returnvalue_3)) (`KismetMathLibrary.RandomFloatInRangeFromStream` (* -1 _returnvalue_2) _returnvalue_2 (`KismetMathLibrary.MakeRandomStream` (`KismetMathLibrary.RandomIntegerInRangeFromStream` 0 1000 (`KismetMathLibrary.MakeRandomStream` _returnvalue_3))))) (`KismetMathLibrary.MakeRotator` 0.0 0.0 (`KismetMathLibrary.RandomFloatInRangeFromStream` 0.0 360.0 _randomstream))))
    (`AddComponent|Static Mesh Component_0` :`RelativeTransform` (`self.TempTransform`))))