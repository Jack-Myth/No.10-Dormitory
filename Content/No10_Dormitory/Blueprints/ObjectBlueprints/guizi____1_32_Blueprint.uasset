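; Lockable cabinet door in the dormitory level that swings open when the player has the required key tag.
; The pickup interface's facing event toggles input, so left click checks the player for TagRequest and shows a key hint if it is missing.
; A one-shot timeline yaws the Axis actor from its construction-time start rotation, with ChangeRot reversing the swing.
; The construction script also sets the actor's tag from PickupTag.
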(event `/Game/No10_Dormitory/Blueprints/PickupsInterface.PickupInterface_ChangeFaceAtObject`
  (params (IsFaceing :type Boolean))
  (bind _returnvalue (`GameplayStatics.GetPlayerController` 0))
  (if IsFaceing
    (`self.EnableInput` _returnvalue)
    (`KismetSystemLibrary.PrintString` "in")
    (else
      (`self.DisableInput` _returnvalue)
      (`KismetSystemLibrary.PrintString` "Out"))))

(event `Key|LeftMouseButton`
  (params (Key :type "Key Structure" :default "AnyKey"))
  (bind _axis (`self.Axis`))
  (:`Pressed`
    (`/Game/No10_Dormitory/Blueprints/GameMacro.FindIfPlayerHaveTag` (`self.TagRequest`)
      (:`Find`
        (`/Engine/EditorBlueprintResources/StandardMacros.DoOnce` false
          (:`Completed`
            (bind (_direction _rot) (`Timeline|时间轴_0` :`NewTime` 1.0 :!label _label)
              (:`Update`
                (if (`self.ChangeRot`)
                  (`self.K2_SetActorRotation` _axis (`KismetMathLibrary.MakeRotator` 0.0 0.0 (+ (`self.StartRot`) (* -1 _rot))) false)
                  (else
                    (`self.K2_SetActorRotation` _axis (`KismetMathLibrary.MakeRotator` 0.0 0.0 (+ (`self.StartRot`) _rot)) false))))))))
      (:`Not`
        (`/Game/No10_Dormitory/Blueprints/GameMacro.ShowMessage` "这个柜子门好像是可以打开的，或许哪里有钥匙？")))))

(event `/Game/No10_Dormitory/Blueprints/PickupsInterface.PickupInterface_OnPicked`
  (goto _label :!via `SetNewTime`))

(fn `UserConstructionScript`
  (bind (_returnvalue_roll _returnvalue_pitch _returnvalue_yaw) (`KismetMathLibrary.BreakRotator` (`self.K2_GetActorRotation` (`self.Axis`))))
  (set `self.Tags` (`|MakeArray` (`KismetStringLibrary.Conv_StringToName` (`self.PickupTag`))))
  (set `self.StartRot` _returnvalue_yaw))