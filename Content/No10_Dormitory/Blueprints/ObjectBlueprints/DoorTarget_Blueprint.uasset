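; Interactable door Blueprint that swings open on a left click when the player holds its required tag.
; The pickup interface enables input while faced; a click searches the character's pickup tags for RequestTag, then adds the door's first actor tag and plays a yaw timeline.
; Switch reverses the swing, and the picked event sets the timeline's time.
; The construction script caches starting yaw and orients a direction arrow, accounting for Switch and negative scale.
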(event `/Game/No10_Dormitory/Blueprints/PickupsInterface.PickupInterface_ChangeFaceAtObject`
  (params (IsFaceing :type Boolean))
  (bind _returnvalue (`GameplayStatics.GetPlayerController` 0))
  ;[1 1 1] Enable And Disable Input
  (if IsFaceing
    (`self.EnableInput` _returnvalue)
    (else
      (`self.DisableInput` _returnvalue))))

(event `Key|LeftMouseButton`
  (params (Key :type "Key Structure" :default "AnyKey"))
  (bind _actorrotationz (`self.ActorRotationZ`))
  (:`Pressed`
    (bind _asmy_character_blueprint (cast `/Game/No10_Dormitory/Blueprints/ObjectBlueprints/MyCharacterBlueprint` (`GameplayStatics.GetPlayerCharacter` 0)))
    (bind _array_element (`/Game/No10_Dormitory/Blueprints/MacroLibrary.ForEachLoopWithBreakOutput` (`/Game/No10_Dormitory/Blueprints/ObjectBlueprints/MyCharacterBlueprint.PickUpTagsData` _asmy_character_blueprint))
      (:`LoopBody`
        (if (`KismetStringLibrary.EqualEqual_StrStr` _array_element (`self.RequestTag`))
          (set `self.FindTag` true)))
      (:`Completed`
        (if (`self.FindTag`)
          (`/Game/No10_Dormitory/Blueprints/GameMacro.AddPickupTag` (`KismetStringLibrary.Conv_NameToString` (`KismetArrayLibrary.Array_Get` (`self.Tags`)))
            (:`Out`
              (bind (_direction `_新建轨迹_0`) (`Timeline|时间轴_0` :`NewTime` 1.0 :!label _label)
                (:`Update`
                  (if (`self.Switch`)
                    (`self.K2_SetActorRotation` (`KismetMathLibrary.MakeRotator` 0.0 0.0 (+ _actorrotationz (* -1 `_新建轨迹_0`))))
                    (else
                      (`self.K2_SetActorRotation` (`KismetMathLibrary.MakeRotator` 0.0 0.0 (+ _actorrotationz `_新建轨迹_0`))))))))))))))

(event `/Game/No10_Dormitory/Blueprints/PickupsInterface.PickupInterface_OnPicked`
  (goto _label :!via `SetNewTime`))

(fn `UserConstructionScript`
  (bind (_returnvalue_roll _returnvalue_pitch _returnvalue_yaw) (`KismetMathLibrary.BreakRotator` (`self.K2_GetActorRotation`)))
  (bind (_returnvalue_x _returnvalue_y _returnvalue_z) (`KismetMathLibrary.BreakVector` (`self.GetActorScale3D`)))
  (bind _arrow1 (`self.Arrow1`))
  (set `self.ActorRotationZ` _returnvalue_yaw)
  (if (xor (or (or (< _returnvalue_x 0.0) (< _returnvalue_y 0.0)) (< _returnvalue_z 0.0)) (`self.Switch`))
    (`SceneComponent.K2_SetRelativeRotation` _arrow1 (struct) false false)
    (else
      (`SceneComponent.K2_SetRelativeRotation` _arrow1 (struct :`Yaw` 180.0) false false))))