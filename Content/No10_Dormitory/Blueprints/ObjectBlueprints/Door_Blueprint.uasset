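; Dormitory door that swings Box1 open or closed on one of two timelines, chosen by Point, via OpenDoor/CloseDoor events or player clicks.
; The pickup interface enables input only while faced; left-click toggles through a FlipFlop if CanBeOpend.
; A set RequestTag adds a player tag check first, though the lookup receives an empty string.
; The construction script shows an optional numbered label with configurable side and text rotation.
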(event `OpenDoor`
  (bind _box1 (`self.Box1`))
  (if (`self.Point`)
    (bind (_direction _tl) (`Timeline|时间轴_0` :!label _label)
      (:`Update`
        (`SceneComponent.K2_SetRelativeRotation` _box1 (`KismetMathLibrary.MakeRotator` 0.0 0.0 _tl) false false)))
    (else
      (bind (_direction_2 _tl_2) (`Timeline|时间轴_1` :!label _label_2)
        (:`Update`
          (`SceneComponent.K2_SetRelativeRotation` _box1 (`KismetMathLibrary.MakeRotator` 0.0 0.0 _tl_2) false false))))))

(event `/Game/No10_Dormitory/Blueprints/PickupsInterface.PickupInterface_ChangeFaceAtObject`
  (params (IsFaceing :type Boolean))
  (bind _returnvalue (`GameplayStatics.GetPlayerController` 0))
  (if IsFaceing
    (`self.EnableInput` _returnvalue)
    (else
      (`self.DisableInput` _returnvalue))))

(event `Key|LeftMouseButton`
  (params (Key :type "Key Structure" :default "AnyKey"))
  (:`Pressed`
    (if (`self.CanBeOpend`)
      (if (`KismetStringLibrary.NotEqual_StrStr` (`self.RequestTag`))
        (`/Game/No10_Dormitory/Blueprints/GameMacro.FindIfPlayerHaveTag` ""
          (:`Find`
            _)))
      (if (`self.Point`)
        (`/Engine/EditorBlueprintResources/StandardMacros.FlipFlop`
          (:`A`
            (goto _label))
          (:`B`
            (goto _label :!via `Reverse`)))
        (else
          (`/Engine/EditorBlueprintResources/StandardMacros.FlipFlop`
            (:`A`
              (goto _label_2))
            (:`B`
              (goto _label_2 :!via `Reverse`))))))))

(event `CloseDoor`
  (if (`self.Point`)
    (goto _label :!via `Reverse`)
    (else
      (goto _label_2 :!via `Reverse`))))

(fn `UserConstructionScript`
  (bind _staticmesh3 (`self.StaticMesh3`))
  (bind _textrender (`self.TextRender`))
  (if (`self.HaveLable`)
    (`SceneComponent.SetVisibility` (`self.StaticMesh3`) true false)
    (`SceneComponent.SetVisibility` (`self.TextRender`) true false)
    (`TextRenderComponent.K2_SetText` (`self.TextRender`) (`KismetTextLibrary.Conv_IntToText` (`self.Number`)))
    (if (`self.SwitchLablePoint`)
      (`SceneComponent.K2_SetRelativeLocationAndRotation` _staticmesh3 (35.0 -0.8 135.0) (struct :`Yaw` 180.0 :`Roll` 90.0) false false)
      (else
        (`SceneComponent.K2_SetRelativeLocationAndRotation` _staticmesh3 (35.0 0.8 135.0) (struct :`Roll` 90.0) false false)))
    (if (`self.TextRot`)
      (`SceneComponent.K2_SetRelativeRotation` _textrender (struct :`Pitch` 90.0 :`Roll` -90.0) false false)
      (else
        (`SceneComponent.K2_SetRelativeRotation` _textrender (struct :`Pitch` -90.0 :`Roll` -90.0) false false)))
    (else
      (`SceneComponent.SetVisibility` (`self.StaticMesh3`) false false)
      (`SceneComponent.SetVisibility` (`self.TextRender`) false false))))