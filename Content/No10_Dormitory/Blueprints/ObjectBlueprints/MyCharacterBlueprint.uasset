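; First-person player character with walk and sprint movement, an animated flashlight with adjustable brightness, and limited-use ice projectile and smoke abilities that update the HUD.
; Sprinting widens the FOV, and looping timers gradually drain max walk speed while running and restore it otherwise, acting as fatigue.
; Movement input also drives footstep audio and run camera shake.
; A timer-driven camera trace notifies actors through the pickup interface when they gain or lose focus.
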(event `OpenFlashLightAnime`
  (`SceneComponent.SetVisibility` (`self.SpotLight`) true false)
  (set `self.IsFlashAnime` true)
  (bind (_direction _updowny _leftrightz) (`Timeline|TimelineOpenFlashLightAnime` :!via `PlayFromStart`)
    (:`Update`
      (`SceneComponent.K2_SetRelativeRotation` (`self.sdt`) (`KismetMathLibrary.MakeRotator` 0.0 _updowny _leftrightz) false false))
    (:`Finished`
      (set `self.IsFlashAnime` false))))

(event `CloseFlashLightAnime`
  (set `self.IsFlashAnime` true)
  (bind (_direction _updowny _leftrightz) (`Timeline|TimelineCloseFlashLightAnime` :!via `PlayFromStart`)
    (:`Update`
      (`SceneComponent.K2_SetRelativeRotation` (`self.sdt`) (`KismetMathLibrary.MakeRotator` 0.0 _updowny _leftrightz) false false))
    (:`Finished`
      (set `self.IsFlashAnime` false)
      (`SceneComponent.SetVisibility` (`self.SpotLight`) false false))))

(event `SaveGame`
  (bind _returnvalue (`GameplayStatics.CreateSaveGameObject` "/Game/No10_Dormitory/Blueprints/SaveGame_Blueprint.SaveGame_Blueprint_C"))
  (`GameplayStatics.SaveGameToSlot` _returnvalue))

(event `Key|F`
  (params (Key :type "Key Structure" :default "AnyKey"))
  (:`Pressed`
    (if (not (`self.IsFlashAnime`))
      (`/Engine/EditorBlueprintResources/StandardMacros.FlipFlop`
        (:`A`
          (`self.CloseFlashLightAnime`))
        (:`B`
          (`self.OpenFlashLightAnime`))))))

(event `Key|LeftShift`
  (params (Key :type "Key Structure" :default "AnyKey"))
  (bind _camera (`self.Camera`))
  (bind _fieldofview (`CameraComponent.FieldOfView` _camera))
  ;[1 1 1] 跑步走+视野变换
  (:`Pressed`
    (set `self.IsRunning` true)
    (set `self.RunningScale` 3.0)
    (`|ExecutionSequence`
      (:`then_0`
        (goto _label_2 :!via `Break`))
      (:`then_1`
        (bind _index (`/Game/No10_Dormitory/Blueprints/MacroLibrary.ForLoopWithDelay` (`KismetMathLibrary.FTrunc` _fieldofview) 105 0.01 :!label _label)
          (:`LoopBody`
            (`CameraComponent.SetFieldOfView` _camera (`KismetMathLibrary.Conv_IntToDouble` _index)))))))
  (:`Released`
    (set `self.IsRunning` false)
    (`|ExecutionSequence`
      (:`then_1`
        (set `self.RunningScale` 1.0)
        (`|ExecutionSequence`
          (:`then_0`
            (goto _label :!via `Break`))
          (:`then_1`
            (bind _index_2 (`/Game/No10_Dormitory/Blueprints/MacroLibrary.ForLoopWithDelay` (- 105 (`KismetMathLibrary.FTrunc` _fieldofview)) 15 0.01 :!label _label_2)
              (:`LoopBody`
                (`CameraComponent.SetFieldOfView` _camera (`KismetMathLibrary.Conv_IntToDouble` (+ (- 15 _index_2) 90)))))))))))

(event `InputAxis|FlashLighting`
  (params (AxisValue :type "Float (single-precision)"))
  (bind _returnvalue (+ AxisValue (`LightComponentBase.Intensity` (`self.SpotLight`))))
  ;[1 1 1] 手电筒亮度
  (if (and (> _returnvalue 0.0) (< _returnvalue 5000.0))
    (`LightComponent.SetIntensity` (`self.SpotLight`) _returnvalue)))

(event `Key|One`
  (params (Key :type "Key Structure" :default "AnyKey"))
  (bind _returnvalue (`GameplayStatics.GetPlayerPawn` 0))
  (bind _bluep_num (`self.BlueP_Num`))
  (bind _returnvalue_2 (`self.GetActorForwardVector` _returnvalue))
  (:`Pressed`
    (if (and (`self.CanUseBlue`) (> _bluep_num 0))
      (`|SpawnActorFromClass` "/Game/No10_Dormitory/Blueprints/ObjectBlueprints/P_Elemental_Ice_Proj_Blueprint.P_Elemental_Ice_Proj_Blueprint_C" (`KismetMathLibrary.MakeTransform` (+ (`self.K2_GetActorLocation` _returnvalue) (* _returnvalue_2 100)) (`KismetMathLibrary.FindLookAtRotation` (`KismetMathLibrary.MakeVector` 0.0) _returnvalue_2)) "Undefined" "OverrideRootScale")
      (`/Engine/EditorBlueprintResources/StandardMacros.DecrementInt` _bluep_num
        (:`  `
          (bind _foundwidgets (`WidgetBlueprintLibrary.GetAllWidgetsOfClass` "/Game/No10_Dormitory/Blueprints/UMG/Main_UMGBlueprint.Main_UMGBlueprint_C"))
          (`/Game/No10_Dormitory/Blueprints/UMG/Main_UMGBlueprint.SetPrower` (`KismetArrayLibrary.Array_Get` _foundwidgets) (`self.BlackP_Num`) _bluep_num))))))

(event `self.ReceiveBeginPlay`
  (`KismetSystemLibrary.K2_SetTimer` null "SendLine" 0.1 true))

(event `Key|Two`
  (params (Key :type "Key Structure" :default "AnyKey"))
  (bind _blackp_num (`self.BlackP_Num`))
  (:`Pressed`
    (if (> _blackp_num 0)
      (`|SpawnActorFromClass` "/Game/No10_Dormitory/Blueprints/ObjectBlueprints/Smoke_Blueprint.Smoke_Blueprint_C" (`KismetMathLibrary.MakeTransform` (`self.K2_GetActorLocation` self) (struct) (1.0 1.0 1.0)) "Undefined" "OverrideRootScale")
      (`/Engine/EditorBlueprintResources/StandardMacros.DecrementInt` _blackp_num
        (:`  `
          (bind _foundwidgets (`WidgetBlueprintLibrary.GetAllWidgetsOfClass` "/Game/No10_Dormitory/Blueprints/UMG/Main_UMGBlueprint.Main_UMGBlueprint_C"))
          (`/Game/No10_Dormitory/Blueprints/UMG/Main_UMGBlueprint.SetPrower` (`KismetArrayLibrary.Array_Get` _foundwidgets) _blackp_num (`self.BlueP_Num`)))))))

(event `InputAxis|Forword`
  (params (AxisValue :type "Float (single-precision)"))
  (bind (_returnvalue_roll _returnvalue_pitch _returnvalue_yaw) (`KismetMathLibrary.BreakRotator` (`self.GetControlRotation`)))
  (bind _returnvalue (`KismetMathLibrary.GetForwardVector` (`KismetMathLibrary.MakeRotator` 0.0 0.0 _returnvalue_yaw)))
  ;[1 1 1] 移动
  (if (`self.IsRunning`)
    (`self.AddMovementInput` _returnvalue (* 3 AxisValue))
    (else
      (`self.AddMovementInput` _returnvalue AxisValue)))
  ;[1 1 1] 脚步声
  (`self.WalkSound` AxisValue (stale `InputAxis|Right` AxisValue) :!label _label_3
    (:`Out`
      (`self.TimerForRun` AxisValue (stale `InputAxis|Right` AxisValue)))))

(event `InputAxis|ViewX`
  (params (AxisValue :type "Float (single-precision)"))
  ;[1 1 1] 视角
  (`self.AddControllerYawInput` AxisValue))

(event `InputAxis|ViewY`
  (params (AxisValue :type "Float (single-precision)"))
  (bind _returnvalue (+ (.pitch (.rotation (`SceneComponent.GetRelativeTransform` (`self.Camera`)))) AxisValue))
  ;[1 1 1] 视角
  (if (not (or (> _returnvalue 60.0) (< _returnvalue -60.0)))
    (`SceneComponent.K2_AddRelativeRotation` (`self.Camera`) (`KismetMathLibrary.MakeRotator` 0.0 AxisValue) false false)))

(event `InputAxis|Right`
  (params (AxisValue :type "Float (single-precision)"))
  (bind (_returnvalue_roll _returnvalue_pitch _returnvalue_yaw) (`KismetMathLibrary.BreakRotator` (`self.GetControlRotation`)))
  (bind _returnvalue (`KismetMathLibrary.GetRightVector` (`KismetMathLibrary.MakeRotator` 0.0 0.0 _returnvalue_yaw)))
  ;[1 1 1] 移动
  (if (`self.IsRunning`)
    (`self.AddMovementInput` _returnvalue (* (`self.RunningScale`) AxisValue))
    (goto _label_3)
    (else
      (`self.AddMovementInput` _returnvalue AxisValue)
      (goto _label_3))))

(fn `SendLine`
  (bind _camera (`self.Camera`))
  (bind _lastfacedactor (`self.LastFacedActor`))
  (bind _returnvalue (`KismetSystemLibrary.IsValid` _lastfacedactor))
  (bind _returnvalue_2 (`SceneComponent.K2_GetComponentLocation` _camera))
  (bind (_outhit _returnvalue_3) (`KismetSystemLibrary.LineTraceSingle` :`Start` _returnvalue_2 :`End` (+ _returnvalue_2 (* (`SceneComponent.GetForwardVector` _camera) 256)) :`TraceChannel` "TraceTypeQuery1" :`DrawTime` 1.0))
  (if _returnvalue_3
    (if (not (== (`.HitActor` (`GameplayStatics.BreakHitResult` _outhit)) _lastfacedactor))
      (if _returnvalue
        (message `/Game/No10_Dormitory/Blueprints/PickupsInterface.PickupInterface_ChangeFaceAtObject` _lastfacedactor false))
      (message `/Game/No10_Dormitory/Blueprints/PickupsInterface.PickupInterface_ChangeFaceAtObject` (`.HitActor` (`GameplayStatics.BreakHitResult` _outhit)) true)
      (set `self.LastFacedActor` (`.HitActor` (`GameplayStatics.BreakHitResult` _outhit))))
    (elif _returnvalue
      (message `/Game/No10_Dormitory/Blueprints/PickupsInterface.PickupInterface_ChangeFaceAtObject` _lastfacedactor false)
      (set `self.LastFacedActor` null))))

(fn `TimerToAddMaxSpeed`
  (bind _charactermovement (`self.CharacterMovement`))
  (bind _returnvalue (+ (`CharacterMovementComponent.MaxWalkSpeed` _charactermovement) 1.0))
  (if (< _returnvalue 600.0)
    (set `CharacterMovementComponent.MaxWalkSpeed` _returnvalue _charactermovement)
    (else
      (`KismetSystemLibrary.K2_ClearTimer` null "TimerToAddMaxSpeed"))))

(fn `TimerToSubMaxSpeed`
  (bind _charactermovement (`self.CharacterMovement`))
  (bind _returnvalue (- (`CharacterMovementComponent.MaxWalkSpeed` _charactermovement) 1.0))
  (if (> _returnvalue 200.0)
    (set `CharacterMovementComponent.MaxWalkSpeed` _returnvalue _charactermovement)
    (else
      (`KismetSystemLibrary.K2_ClearTimer` null "TimerToSubMaxSpeed"))))

(fn `UserConstructionScript`)