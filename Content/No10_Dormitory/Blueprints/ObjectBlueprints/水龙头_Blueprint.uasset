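; Interactable dormitory faucet Blueprint that a player toggles open and closed with left click while facing it, with input enabled and disabled through the pickup interface.
; Clicks require a player tag check and CanBeUsed, and closing also requires CanBeClosed.
; A timeline rotates the mesh's yaw from its construction-time angle.
; Its first completion fires a named event via the "ce" console command and adds the first pickup tag, guarded by DoOnce.
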(event `/Game/No10_Dormitory/Blueprints/PickupsInterface.PickupInterface_ChangeFaceAtObject`
  (params (IsFaceing :type Boolean))
  (bind _returnvalue (`GameplayStatics.GetPlayerController` 0))
  (if IsFaceing
    (`self.EnableInput` _returnvalue)
    (`KismetSystemLibrary.PrintString` "In")
    (else
      (`self.DisableInput` _returnvalue)
      (`KismetSystemLibrary.PrintString` "Out"))))

(event `Key|LeftMouseButton`
  (params (Key :type "Key Structure" :default "AnyKey"))
  (:`Pressed`
    (`/Game/No10_Dormitory/Blueprints/GameMacro.FindIfPlayerHaveTag` (`self.RequestTag`)
      (:`Find`
        (if (`self.CanBeUsed`)
          (if (`self.IsOpend`)
            (if (`self.CanBeClosed`)
              (set `self.IsOpend` false)
              (bind (_direction `_新建轨迹_0`) (`Timeline|时间轴_0` :!via `Reverse` :!label _label)
                (:`Update`
                  (`SceneComponent.K2_SetRelativeRotation` (`self.StaticMeshComponent01`) (`KismetMathLibrary.MakeRotator` 0.0 0.0 (+ (`self.StartRotation`) `_新建轨迹_0`)) false false))
                (:`Finished`
                  (`/Engine/EditorBlueprintResources/StandardMacros.DoOnce` false
                    (:`Completed`
                      (`KismetSystemLibrary.ExecuteConsoleCommand` (`KismetStringLibrary.Concat_StrStr` "ce " (`self.EventNameAfterOpend`)))
                      (`/Game/No10_Dormitory/Blueprints/GameMacro.AddPickupTag` (`KismetStringLibrary.Conv_NameToString` (`KismetArrayLibrary.Array_Get` (`self.Tags`)))))))))
            (else
              (set `self.IsOpend` true)
              (goto _label))))))))

(fn `UserConstructionScript`
  (set `self.StartRotation` (.yaw (.rotation (`SceneComponent.GetRelativeTransform` (`self.StaticMeshComponent01`))))))