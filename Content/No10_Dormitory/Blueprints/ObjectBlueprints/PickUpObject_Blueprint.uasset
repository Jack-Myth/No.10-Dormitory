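; Base pickup object that the player collects with right mouse while facing it, or that shows a message when it cannot be picked.
; An interface event toggles its input as focus changes; picking records the tag on the character, plays a sound and can open a paused information widget.
; Configurable level-script events fire through "ce" console commands before and after pickup, after which the object hides and drops collision.
; The construction script sets the actor tag and optional helper box.
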(event `/Game/No10_Dormitory/Blueprints/PickupsInterface.PickupInterface_ChangeFaceAtObject`
  (params (IsFaceing :type Boolean))
  (bind _returnvalue (`GameplayStatics.GetPlayerController` 0))
  ;[1 1 1] Enable And Disable Input
  (if IsFaceing
    (`self.EnableInput` _returnvalue)
    (`KismetSystemLibrary.PrintString` "In")
    (else
      (`self.DisableInput` _returnvalue)
      (`KismetSystemLibrary.PrintString` "Out"))))

(event `Pick`
  (bind _returnvalue (`GameplayStatics.GetPlayerController` 0))
  ;[1 1 1] Action Before Object Picked
  (bind _asmy_character_blueprint (cast `/Game/No10_Dormitory/Blueprints/ObjectBlueprints/MyCharacterBlueprint` (`GameplayStatics.GetPlayerCharacter` 0) :!label _label)) ; 嘿嘿嘿嘿。。。。
  (`KismetArrayLibrary.Array_Add` (`/Game/No10_Dormitory/Blueprints/ObjectBlueprints/MyCharacterBlueprint.PickUpTagsData` _asmy_character_blueprint) (`self.PickUpTag`)) ; 好大一个add。。
  (`GameplayStatics.PlaySoundAtLocation` (`self.PickUpSound`) (`self.K2_GetActorLocation`) :!label _label_2) ; 放一个声音在他的位置？
  (`KismetSystemLibrary.ExecuteConsoleCommand` (`KismetStringLibrary.Concat_StrStr` "ce " (`self.EventBeforePicked`))) ; 我也听到
  (if (`self.ShowObjectInformation`)
    (bind _foundwidgets (`WidgetBlueprintLibrary.GetAllWidgetsOfClass` "/Game/No10_Dormitory/Blueprints/UMG/NewObjectWidgetBlueprint.NewObjectWidgetBlueprint_C"))
    (bind _item (`KismetArrayLibrary.Array_Get` _foundwidgets))
    (`/Game/No10_Dormitory/Blueprints/UMG/NewObjectWidgetBlueprint.SetNewObject` _item (`self.ObjectImage`) (`self.ObjectTitle`) (`self.ObjectInformation`))
    (`/Game/No10_Dormitory/Blueprints/UMG/NewObjectWidgetBlueprint.StartFadeIn` _item false null)
    (`GameplayStatics.SetGamePaused` true)
    (`WidgetBlueprintLibrary.SetInputMode_UIOnlyEx` _returnvalue _item)
    (set `PlayerController.bShowMouseCursor` true _returnvalue))
  (message `/Game/No10_Dormitory/Blueprints/PickupsInterface.PickupInterface_OnPicked` self))

(event `Key|RightMouseButton`
  (params (Key :type "Key Structure" :default "AnyKey"))
  (bind _cantpickinformation (`self.CantPickInformation`))
  ;[1 1 1] Action Before Object Picked
  (:`Pressed`
    (if (`self.CanBePicked`)
      (if (`KismetStringLibrary.NotEqual_StrStr` (`self.PickUpTag`))
        (goto _label)
        (else
          (goto _label_2)))
      (elif (`KismetStringLibrary.NotEqual_StrStr` _cantpickinformation)
        (`/Game/No10_Dormitory/Blueprints/GameMacro.ShowMessage` _cantpickinformation)))))

(event `/Game/No10_Dormitory/Blueprints/PickupsInterface.PickupInterface_OnPicked`
  ;[1 1 1] Action After Picked
  (`KismetSystemLibrary.ExecuteConsoleCommand` (`KismetStringLibrary.Concat_StrStr` "ce " (`self.EventAfterPicked`)))
  (`self.SetActorHiddenInGame` true)
  (`PrimitiveComponent.SetCollisionEnabled` (`self.Box`) "NoCollision")
  (`PrimitiveComponent.SetCollisionEnabled` (`self.StaticMeshComponent`) "NoCollision"))

(event `ShowPickupInformations`
  (params (Button :type "/Game/No10_Dormitory/Blueprints/UMG/ScanPickupObjectWidgetBlueprint Object Reference"))
  (bind _foundwidgets (`WidgetBlueprintLibrary.GetAllWidgetsOfClass` "/Game/No10_Dormitory/Blueprints/UMG/NewObjectWidgetBlueprint.NewObjectWidgetBlueprint_C"))
  (bind _item (`KismetArrayLibrary.Array_Get` _foundwidgets))
  (`/Game/No10_Dormitory/Blueprints/UMG/NewObjectWidgetBlueprint.SetNewObject` _item (`self.ObjectImage`) (`self.ObjectTitle`) (`self.ObjectInformation`))
  (`/Game/No10_Dormitory/Blueprints/UMG/NewObjectWidgetBlueprint.StartFadeIn` _item true Button))

(fn `UserConstructionScript`
  (bind _havehelpfulboxcollision (`self.HaveHelpfulBoxCollision`))
  (`SceneComponent.SetVisibility` (`self.Box`) _havehelpfulboxcollision false)
  (if (not _havehelpfulboxcollision)
    (`PrimitiveComponent.SetCollisionEnabled` (`self.Box`) "NoCollision"))
  (set `self.Tags` (`|MakeArray` (`KismetStringLibrary.Conv_StringToName` (`self.PickUpTag`)))))