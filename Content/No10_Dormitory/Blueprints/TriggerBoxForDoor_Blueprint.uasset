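; Trigger box for a door in the dormitory level that lets the player swing a Door actor open and closed.
; Overlap begin and end enable and disable player input on the trigger, so left mouse clicks count only nearby.
; Each click alternates a timeline between play and reverse through a FlipFlop.
; The timeline sets the door's yaw to Start plus EndStep scaled by its curve, keeping roll and pitch.
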(event `self.CollisionComponent.OnComponentBeginOverlap`
  (params (OverlappedComponent :type "PrimitiveComponent Object Reference") (OtherActor :type "Actor Object Reference") (OtherComp :type "PrimitiveComponent Object Reference") (OtherBodyIndex :type Integer) (bFromSweep :type Boolean) (SweepResult :type "HitResult Structure (by ref)"))
  (`self.EnableInput` (`GameplayStatics.GetPlayerController` 0)))

(event `Key|LeftMouseButton`
  (params (Key :type "Key Structure" :default "AnyKey"))
  (bind _door (`self.Door`))
  (bind (_returnvalue_roll _returnvalue_pitch) (`KismetMathLibrary.BreakRotator` (`self.K2_GetActorRotation` _door)))
  (:`Pressed`
    (`/Engine/EditorBlueprintResources/StandardMacros.FlipFlop`
      (:`A`
        (bind (_direction _0_90) (`Timeline|时间轴_0` :!label _label)
          (:`Update`
            (`self.K2_SetActorRotation` _door (`KismetMathLibrary.MakeRotator` _returnvalue_roll _returnvalue_pitch (+ (`self.Start`) (* (`self.EndStep`) _0_90))) false))))
      (:`B`
        (goto _label :!via `Reverse`)))))

(event `self.CollisionComponent.OnComponentEndOverlap`
  (params (OverlappedComponent :type "PrimitiveComponent Object Reference") (OtherActor :type "Actor Object Reference") (OtherComp :type "PrimitiveComponent Object Reference") (OtherBodyIndex :type Integer))
  (`self.DisableInput` (`GameplayStatics.GetPlayerController` 0)))

(fn `UserConstructionScript`)