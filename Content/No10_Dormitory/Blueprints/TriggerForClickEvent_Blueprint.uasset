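; Clickable trigger actor that fires a named custom event through the "ce" console command when clicked.
; A pickup-interface facing event enables input only while the object is faced, and SetClickable toggles left and right click separately.
; Both buttons share one path, which adds the click tag once, runs the command and optionally destroys the actor.
; Construction sets the actor's tag from ClickTag.
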(event `/Game/No10_Dormitory/Blueprints/PickupsInterface.PickupInterface_ChangeFaceAtObject`
  (params (IsFaceing :type Boolean))
  (bind _returnvalue (`GameplayStatics.GetPlayerController` 0))
  (if IsFaceing
    (`self.EnableInput` _returnvalue)
    (else
      (`self.DisableInput` _returnvalue))))

(event `Key|LeftMouseButton`
  (params (Key :type "Key Structure" :default "AnyKey"))
  (:`Pressed`
    (if (`self.CanBeLeftClick`)
      (`|ExecutionSequence` :!label _label
        (:`then_0`
          (`/Engine/EditorBlueprintResources/StandardMacros.DoOnce` false
            (:`Completed`
              (`/Game/No10_Dormitory/Blueprints/GameMacro.AddPickupTag` (`self.ClickTag`)))))
        (:`then_1`
          (`KismetSystemLibrary.ExecuteConsoleCommand` (`KismetStringLibrary.Concat_StrStr` "ce " (`self.ClickEventName`)))
          (if (`self.AutoDestroy`)
            (`self.K2_DestroyActor`)))))))

(event `Key|RightMouseButton`
  (params (Key :type "Key Structure" :default "AnyKey"))
  (:`Pressed`
    (if (`self.CanBeRightClick`)
      (goto _label))))

(event `SetClickable`
  (params (Left :type Boolean) (Right :type Boolean))
  (set `self.CanBeLeftClick` Left)
  (set `self.CanBeRightClick` Right))

(fn `UserConstructionScript`
  (set `self.Tags` (`|MakeArray` (`KismetStringLibrary.Conv_StringToName` (`self.ClickTag`)))))