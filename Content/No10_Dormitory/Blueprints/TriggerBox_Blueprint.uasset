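; Trigger box that lets the player fire named custom events with the left and right mouse buttons while overlapping it.
; Overlap begin enables input for player controller 0 and overlap end disables it, with no check on the overlapping actor.
; Each click appends its button's event-name variable to "ce" and runs it as a console command, invoking Level Blueprint events without direct references.
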(event `self.CollisionComponent.OnComponentBeginOverlap`
  (params (OverlappedComponent :type "PrimitiveComponent Object Reference") (OtherActor :type "Actor Object Reference") (OtherComp :type "PrimitiveComponent Object Reference") (OtherBodyIndex :type Integer) (bFromSweep :type Boolean) (SweepResult :type "HitResult Structure (by ref)"))
  (`self.EnableInput` (`GameplayStatics.GetPlayerController` 0)))

(event `Key|LeftMouseButton`
  (params (Key :type "Key Structure" :default "AnyKey"))
  (:`Pressed`
    (`KismetSystemLibrary.ExecuteConsoleCommand` (`KismetStringLibrary.Concat_StrStr` "ce " (`self.LeftButtonEvent`)))))

(event `self.CollisionComponent.OnComponentEndOverlap`
  (params (OverlappedComponent :type "PrimitiveComponent Object Reference") (OtherActor :type "Actor Object Reference") (OtherComp :type "PrimitiveComponent Object Reference") (OtherBodyIndex :type Integer))
  (`self.DisableInput` (`GameplayStatics.GetPlayerController` 0)))

(event `Key|RightMouseButton`
  (params (Key :type "Key Structure" :default "AnyKey"))
  (:`Pressed`
    (`KismetSystemLibrary.ExecuteConsoleCommand` (`KismetStringLibrary.Concat_StrStr` "ce " (`self.RightButtonEvent`)))))

(fn `UserConstructionScript`)