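; Breakable dormitory door, with an optional numbered label plate placed and oriented by the construction script.
; Pickup-interface facing toggles input; a left click checks the player for the required tag, adds the door's own tag and breaks it once.
; Breaking, also triggered directly by the picked event, spawns a randomly rotated physics mesh, then after a short delay hides a door mesh and disables blocking collision.
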(event `/Game/No10_Dormitory/Blueprints/PickupsInterface.PickupInterface_ChangeFaceAtObject`
  (params (IsFaceing :type Boolean))
  (bind _returnvalue (`GameplayStatics.GetPlayerController` 0))
  (if IsFaceing
    (`self.EnableInput` _returnvalue)
    (else
      (`self.DisableInput` _returnvalue))))

(event `Key|LeftMouseButton`
  (params (Key :type "Key Structure" :default "AnyKey"))
  (:`Pressed`
    (`/Game/No10_Dormitory/Blueprints/GameMacro.FindIfPlayerHaveTag` (`self.RequestTag`)
      (:`Find`
        (`/Game/No10_Dormitory/Blueprints/GameMacro.AddPickupTag` (`KismetStringLibrary.Conv_NameToString` (`KismetArrayLibrary.Array_Get` (`self.Tags`)))
          (:`Out`
            (`/Engine/EditorBlueprintResources/StandardMacros.DoOnce` false
              (:`Completed`
                (bind _returnvalue (`|SpawnActorFromClass` "/Game/No10_Dormitory/Blueprints/ObjectBlueprints/MoveableStaticMeshActor.MoveableStaticMeshActor_C" (`KismetMathLibrary.MakeTransform` (`SceneComponent.K2_GetComponentLocation` (`self.Scene`)) (`KismetMathLibrary.RandomRotator` true)) "AdjustIfPossibleButAlwaysSpawn" "OverrideRootScale" :!label _label))
                (bind _staticmeshcomponent (`StaticMeshActor.StaticMeshComponent` _returnvalue))
                (`StaticMeshComponent.SetStaticMesh` _staticmeshcomponent "/Game/No10_Dormitory/StaticMesh/Tongzhuangshui.Tongzhuangshui")
                (`PrimitiveComponent.SetSimulatePhysics` _staticmeshcomponent true)
                (`KismetSystemLibrary.Delay` 0.5)
                (`SceneComponent.SetVisibility` (`self.StaticMesh2`) false false)
                (`PrimitiveComponent.SetCollisionResponseToChannel` _staticmeshcomponent "ECC_Pawn" "ECR_Ignore")
                (`PrimitiveComponent.SetCollisionEnabled` (`self.StaticMesh3`) "NoCollision")
                (`PrimitiveComponent.SetCollisionEnabled` (`self.StaticMesh2`) "NoCollision")
                (`PrimitiveComponent.SetCollisionEnabled` (`self.Cube_DM`) "NoCollision")))))))))

(event `/Game/No10_Dormitory/Blueprints/PickupsInterface.PickupInterface_OnPicked`
  (goto _label))

(fn `UserConstructionScript`
  (bind _staticmesh3 (`self.StaticMesh3`))
  (bind _textrender (`self.TextRender`))
  (if (`self.HaveLable`)
    (`SceneComponent.SetVisibility` (`self.StaticMesh3`) true false)
    (`SceneComponent.SetVisibility` (`self.TextRender`) true false)
    (`TextRenderComponent.K2_SetText` (`self.TextRender`) (`KismetTextLibrary.Conv_IntToText` (`self.Number`)))
    (if (`self.SwitchLablePoint`)
      (`SceneComponent.K2_SetRelativeLocationAndRotation` _staticmesh3 (35.0 -0.8 135.0) (struct :`Yaw` 180.0 :`Roll` 90.0) false false)
      (else
        (`SceneComponent.K2_SetRelativeLocationAndRotation` _staticmesh3 (35.0 0.8 135.0) (struct :`Roll` 90.0) false false)))
    (if (`self.TextRot`)
      (`SceneComponent.K2_SetRelativeRotation` _textrender (struct :`Pitch` 90.0 :`Roll` -90.0) false false)
      (else
        (`SceneComponent.K2_SetRelativeRotation` _textrender (struct :`Pitch` -90.0 :`Roll` -90.0) false false)))
    (else
      (`SceneComponent.SetVisibility` (`self.StaticMesh3`) false false)
      (`SceneComponent.SetVisibility` (`self.TextRender`) false false))))