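; An interactive object Blueprint that accepts player input while faced, spawning physics props and hiding a profane keyboard easter egg.
; A State counter tracks the F-U-C-K-Q sequence, whose completion swaps its mesh, enables physics and calls SexGirl on FunnyCharacterBlueprint.
; The 0 key drops a simulated mesh actor from above at a random horizontal offset, using the alternate mesh while the unlocked state holds.
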(event `/Game/No10_Dormitory/Blueprints/PickupsInterface.PickupInterface_ChangeFaceAtObject`
  (params (IsFaceing :type Boolean))
  (bind _returnvalue (`GameplayStatics.GetPlayerController` 0))
  (if IsFaceing
    (`self.EnableInput` _returnvalue)
    (else
      (`self.DisableInput` _returnvalue))))

(event `Key|F`
  (params (Key :type "Key Structure" :default "AnyKey"))
  (:`Pressed`
    (if (== (`self.State`) 0)
      (set `self.State` 1)
      (else
        (set `self.State` 0)))))

(event `Key|U`
  (params (Key :type "Key Structure" :default "AnyKey"))
  (:`Pressed`
    (if (== (`self.State`) 1)
      (set `self.State` 2)
      (else
        (set `self.State` 0)))))

(event `Key|Zero`
  (params (Key :type "Key Structure" :default "AnyKey"))
  (bind (_returnvalue_x _returnvalue_y _returnvalue_z) (`KismetMathLibrary.BreakVector` (`self.K2_GetActorLocation`)))
  (:`Pressed`
    (bind _returnvalue (`|SpawnActorFromClass` "/Game/No10_Dormitory/Blueprints/ObjectBlueprints/MoveableStaticMeshActor.MoveableStaticMeshActor_C" (`KismetMathLibrary.MakeTransform` (`KismetMathLibrary.MakeVector` (+ _returnvalue_x (`KismetMathLibrary.RandomFloatInRange` -800.0 800.0)) (+ _returnvalue_y (`KismetMathLibrary.RandomFloatInRange` -800.0 800.0)) (+ _returnvalue_z 1000.0))) "Undefined" "OverrideRootScale"))
    (if (== (`self.State`) 5)
      (bind _staticmeshcomponent (`StaticMeshActor.StaticMeshComponent` _returnvalue))
      (`StaticMeshComponent.SetStaticMesh` _staticmeshcomponent "/Game/MyHouse/StaticMesh/2.2")
      (else
        (`StaticMeshComponent.SetStaticMesh` _staticmeshcomponent "/Game/MyHouse/StaticMesh/0.0")))
    (`PrimitiveComponent.SetSimulatePhysics` _staticmeshcomponent true)))

(event `Key|C`
  (params (Key :type "Key Structure" :default "AnyKey"))
  (:`Pressed`
    (if (== (`self.State`) 2)
      (set `self.State` 3)
      (else
        (set `self.State` 0)))))

(event `Key|K`
  (params (Key :type "Key Structure" :default "AnyKey"))
  (:`Pressed`
    (if (== (`self.State`) 3)
      (set `self.State` 4)
      (else
        (set `self.State` 0)))))

(event `Key|Q`
  (params (Key :type "Key Structure" :default "AnyKey"))
  (:`Pressed`
    (if (== (`self.State`) 4)
      (`StaticMeshComponent.SetStaticMesh` (`self.StaticMeshComponent`) "/Game/MyHouse/StaticMesh/2.2")
      (`PrimitiveComponent.SetSimulatePhysics` (`self.StaticMeshComponent`) true)
      (bind _asfunny_character_blueprint (cast `/Game/No10_Dormitory/Blueprints/ObjectBlueprints/FunnyCharacterBlueprint` (`GameplayStatics.GetPlayerCharacter` 0)))
      (`/Game/No10_Dormitory/Blueprints/ObjectBlueprints/FunnyCharacterBlueprint.SexGirl` _asfunny_character_blueprint)
      (set `self.State` 5)
      (else
        (set `self.State` 0)))))

(fn `UserConstructionScript`)